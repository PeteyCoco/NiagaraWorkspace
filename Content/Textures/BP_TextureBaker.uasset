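; BP_TextureBaker is an editor utility Blueprint that bakes a material into a static texture asset.
; Its BakeTexture function checks that a render target and material are set, draws the material into the target, then saves it as a Texture2D named TextureFromRenderTarget.
; The save step is editor-only, and the event graph and construction script are empty.
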(fn `BakeTexture`
  (if (and (`KismetSystemLibrary.IsValid` (`self.Render Target to Draw`)) (`KismetSystemLibrary.IsValid` (`self.Material to Draw From`)))
    (`KismetRenderingLibrary.DrawMaterialToRenderTarget` (`self.Render Target to Draw`) (`self.Material to Draw From`))
    (`KismetRenderingLibrary.RenderTargetCreateStaticTexture2DEditorOnly` (`self.Render Target to Draw`) "TextureFromRenderTarget")))

(fn `UserConstructionScript`)